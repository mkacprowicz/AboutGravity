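; AI controller for BP_EnemyChar1 that runs the enemy behavior tree and feeds it player sightings.
; On possess it caches the pawn and starts EnemyTree.
; Perception updates on the main character set CanSeePlayer; losing sight also stores the player's current location and sets RecentlySighted.
; Walk, Run and Attack events forward to the possessed enemy character.
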(event OnTargetPerceptionUpdated(AIPerception)
  (params (Actor :type Actor%20Object%20Reference) (Stimulus :type AI%20Stimulus%20Structure))
  (bind _bsuccessfullysensed (Utilities|Struct|BreakAIStimulus Stimulus))
  (bind _returnvalue (AI|GetBlackboard 0))
  (Utilities|Casting|CastToBP_MainCharacter Actor)
  (AI|Components|Blackboard|SetValueasBool _returnvalue (Utilities|Name|MakeLiteralName "CanSeePlayer") _bsuccessfullysensed)
  (if (not _bsuccessfullysensed)
    (AI|Components|Blackboard|SetValueasVector _returnvalue (Utilities|Name|MakeLiteralName "PlayerLocation") (Transformation|GetActorLocation (Game|GetPlayerCharacter 0)))
    (AI|Components|Blackboard|SetValueasBool _returnvalue (Utilities|Name|MakeLiteralName "RecentlySighted") true)))

(event Custom|Run
  (Default|Run (Variables|Default|GetEnemyValue)))

(event Custom|Walk
  (Default|Walk (Variables|Default|GetEnemyValue)))

(event Custom|Attack
  (Default|Attack (Variables|Default|GetEnemyValue)))

(event EventPossess
  (params (PossessedPawn :type Pawn%20Object%20Reference))
  (bind _asbp_enemy_char_1 (Utilities|Casting|CastToBP_EnemyChar1 PossessedPawn))
  (Variables|Default|SetEnemyValue _asbp_enemy_char_1)
  (AI|RunBehaviorTree "/Game/Blueprints/Enemy/EnemyTree.EnemyTree"))

(fn ConstructionScript)