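; BP_StreamingLevelTrigger is a trigger volume that streams levels in and out when the player character enters it.
; On Box overlap by BP_PlayerCharacter, it asynchronously loads LevelToLoad, visible once loaded, then requests an asynchronous unload of LevelToUnload.
; Either step is skipped when its level name is None or that level is already in the desired loaded state.
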(event OnComponentBeginOverlap(Box)
  (params (OverlappedComponent :type Primitive%20Component%20Object%20Reference) (OtherActor :type Actor%20Object%20Reference) (OtherComp :type Primitive%20Component%20Object%20Reference) (OtherBodyIndex :type Integer) (bFromSweep :type Boolean) (SweepResult :type Hit%20Result%20Structure%20%28by%20ref%29))
  (bind _leveltoload (Variables|Default|GetLevelToLoad))
  (bind _leveltounload (Variables|Default|GetLevelToUnload))
  (Utilities|Casting|CastToBP_PlayerCharacter OtherActor)
  (Utilities|FlowControl|Sequence
    (:then_0
      (if (not (Utilities|Name|Equal(Name) _leveltoload "None"))
        (if (not (Class|LevelStreaming|IsLevelLoaded (Class|GameplayStatics|GetStreamingLevel _leveltoload)))
          (Game|LoadStreamLevel(byName) _leveltoload true))))
    (:then_1
      (if (not (Utilities|Name|Equal(Name) _leveltounload "None"))
        (if (Class|LevelStreaming|IsLevelLoaded (Class|GameplayStatics|GetStreamingLevel _leveltounload))
          (Game|UnloadStreamLevel(byName) _leveltounload false))))))

(fn ConstructionScript)