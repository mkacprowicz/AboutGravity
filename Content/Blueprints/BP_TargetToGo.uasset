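; BP_TargetToGo is a waypoint actor that passes the player character its next goal when the player overlaps its box.
; It searches all BP_TargetToGo actors for the one whose Index matches its own NextIndex and sends that location to BP_PlayerCharacter through SetNewGoal.
; With no match, it sends the zero vector instead.
; Either way, it hides itself in game, leaving collision untouched.
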(event OnComponentBeginOverlap(Box)
  (params (OverlappedComponent :type Primitive%20Component%20Object%20Reference) (OtherActor :type Actor%20Object%20Reference) (OtherComp :type Primitive%20Component%20Object%20Reference) (OtherBodyIndex :type Integer) (bFromSweep :type Boolean) (SweepResult :type Hit%20Result%20Structure%20%28by%20ref%29))
  (bind _asbp_player_character (Utilities|Casting|CastToBP_PlayerCharacter OtherActor))
  (Variables|Default|SetWasChanged false)
  (bind _outactors (Actor|GetAllActorsOfClass "BP_TargetToGo_C"))
  (bind _array_element (Utilities|Array|ForEachLoopwithBreak _outactors)
    (:LoopBody
      (if (== (Variables|BP_TargetToGo_C|GetIndex _array_element) (Variables|Default|GetNextIndex))
        (Default|SetNewGoal _asbp_player_character (Transformation|GetActorLocation _array_element))
        (Variables|Default|SetWasChanged true)
        (Rendering|SetActorHiddenInGame true)
        (CallFunction|BreakLoop)))
    (:Completed
      (if (not (Variables|Default|GetWasChanged))
        (Default|SetNewGoal _asbp_player_character "0, 0, 0")
        (Rendering|SetActorHiddenInGame true)))))

(event Custom|BreakLoop
  (Utilities|Array|ForEachLoopwithBreak (stale OnComponentBeginOverlap(Box) _outactors)) ; enters at Break
)

(event EventBeginPlay)

(fn ConstructionScript)