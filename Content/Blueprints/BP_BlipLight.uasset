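; BP_BlipLight is a point light that flickers and then swaps between white and green.
; BeginPlay sets the starting colour from the WhiteOne boolean.
; StartFlicker, not called within this Blueprint, reapplies that colour, then runs a hard-coded Delay chain of visibility blinks that come progressively faster.
; On the last blink it inverts WhiteOne and shows the light in the new colour, so each completed sequence alternates the colour.
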(event Custom|StartFlicker
  (bind _pointlight (Variables|Default|GetPointLight))
  (bind _pointlight_2 (Variables|Default|GetPointLight))
  (if (Variables|Default|GetWhiteOne)
    (Rendering|Components|Light|SetLightColor _pointlight "(R=1.000000,G=1.000000,B=1.000000,A=1.000000)" true)
    (else
      (Rendering|Components|Light|SetLightColor _pointlight "(R=0.068225,G=1.000000,B=0.000000,A=1.000000)" true)))
  (Rendering|SetVisibility (Variables|Default|GetPointLight) false false)
  (Utilities|FlowControl|Delay 0.2)
  (Rendering|SetVisibility (Variables|Default|GetPointLight) true false)
  (Utilities|FlowControl|Delay 2.0)
  (Rendering|SetVisibility (Variables|Default|GetPointLight) false false)
  (Utilities|FlowControl|Delay 0.2)
  (Rendering|SetVisibility (Variables|Default|GetPointLight) true false)
  (Utilities|FlowControl|Delay 1.5)
  (Rendering|SetVisibility (Variables|Default|GetPointLight) false false)
  (Utilities|FlowControl|Delay 0.2)
  (Rendering|SetVisibility (Variables|Default|GetPointLight) true false)
  (Utilities|FlowControl|Delay 1.0)
  (Rendering|SetVisibility (Variables|Default|GetPointLight) false false)
  (Utilities|FlowControl|Delay 0.2)
  (Rendering|SetVisibility (Variables|Default|GetPointLight) true false)
  (Utilities|FlowControl|Delay 0.3)
  (Rendering|SetVisibility (Variables|Default|GetPointLight) false false)
  (Utilities|FlowControl|Delay 0.2)
  (Rendering|SetVisibility (Variables|Default|GetPointLight) true false)
  (Utilities|FlowControl|Delay 0.3)
  (Rendering|SetVisibility (Variables|Default|GetPointLight) false false)
  (Utilities|FlowControl|Delay 0.2)
  (Rendering|SetVisibility (Variables|Default|GetPointLight) true false)
  (Utilities|FlowControl|Delay 0.3)
  (Rendering|SetVisibility (Variables|Default|GetPointLight) false false)
  (Variables|Default|SetWhiteOne (not (Variables|Default|GetWhiteOne)))
  (if (Variables|Default|GetWhiteOne)
    (Rendering|Components|Light|SetLightColor _pointlight_2 "(R=1.000000,G=1.000000,B=1.000000,A=1.000000)" true)
    (else
      (Rendering|Components|Light|SetLightColor _pointlight_2 "(R=0.068225,G=1.000000,B=0.000000,A=1.000000)" true)))
  (Rendering|SetVisibility (Variables|Default|GetPointLight) true false))

(event EventBeginPlay
  (bind _pointlight (Variables|Default|GetPointLight))
  (if (Variables|Default|GetWhiteOne)
    (Rendering|Components|Light|SetLightColor _pointlight "(R=1.000000,G=1.000000,B=1.000000,A=1.000000)" true)
    (else
      (Rendering|Components|Light|SetLightColor _pointlight "(R=0.068225,G=1.000000,B=0.000000,A=1.000000)" true))))

(fn ConstructionScript)