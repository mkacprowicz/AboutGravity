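; Sliding door that opens when the player character enters its trigger and closes when they leave.
; Overlap events set Opening or Closing flags, and Tick moves Box along local Y by Speed per frame, unscaled by delta time, between its starting Y and DestinationYValue.
; StopDoor makes the trigger ignore further overlaps and turns the door's lights red, but leaves any movement already underway running.
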(event OnComponentBeginOverlap(Trigger)
  (params (OverlappedComponent :type Primitive%20Component%20Object%20Reference) (OtherActor :type Actor%20Object%20Reference) (OtherComp :type Primitive%20Component%20Object%20Reference) (OtherBodyIndex :type Integer) (bFromSweep :type Boolean) (SweepResult :type Hit%20Result%20Structure%20%28by%20ref%29))
  (Utilities|Casting|CastToBP_PlayerCharacter OtherActor)
  (if (not (Variables|Default|GetDoorStopped))
    (CallFunction|OpenDoor)))

(event OnComponentEndOverlap(Trigger)
  (params (OverlappedComponent :type Primitive%20Component%20Object%20Reference) (OtherActor :type Actor%20Object%20Reference) (OtherComp :type Primitive%20Component%20Object%20Reference) (OtherBodyIndex :type Integer))
  (Utilities|Casting|CastToBP_PlayerCharacter OtherActor)
  (if (not (Variables|Default|GetDoorStopped))
    (CallFunction|CloseDoor)))

(event Custom|OpenDoor
  (Variables|Default|SetOpening true)
  (Variables|Default|SetClosing false))

(event Custom|CloseDoor
  (Variables|Default|SetClosing true)
  (Variables|Default|SetOpening false))

(event Custom|StopDoor
  (Variables|Default|SetDoorStopped true)
  (Rendering|Material|SetMaterial (Variables|Default|GetLight1) 0 "/Game/Mats/RedWall.RedWall")
  (Rendering|Material|SetMaterial (Variables|Default|GetLight10) 0 "/Game/Mats/RedWall.RedWall")
  (Rendering|Material|SetMaterial (Variables|Default|GetLight11) 0 "/Game/Mats/RedWall.RedWall")
  (Rendering|Material|SetMaterial (Variables|Default|GetLight12) 0 "/Game/Mats/RedWall.RedWall")
  (Rendering|Material|SetMaterial (Variables|Default|GetLight2) 0 "/Game/Mats/RedWall.RedWall")
  (Rendering|Material|SetMaterial (Variables|Default|GetLight3) 0 "/Game/Mats/RedWall.RedWall")
  (Rendering|Material|SetMaterial (Variables|Default|GetLight4) 0 "/Game/Mats/RedWall.RedWall")
  (Rendering|Material|SetMaterial (Variables|Default|GetLight5) 0 "/Game/Mats/RedWall.RedWall")
  (Rendering|Material|SetMaterial (Variables|Default|GetLight6) 0 "/Game/Mats/RedWall.RedWall")
  (Rendering|Material|SetMaterial (Variables|Default|GetLight7) 0 "/Game/Mats/RedWall.RedWall")
  (Rendering|Material|SetMaterial (Variables|Default|GetLight8) 0 "/Game/Mats/RedWall.RedWall")
  (Rendering|Material|SetMaterial (Variables|Default|GetLight9) 0 "/Game/Mats/RedWall.RedWall"))

(event EventTick
  (params (DeltaSeconds :type Float%20%28single-precision%29))
  (if (Variables|Default|GetOpening)
    (if (<= (.y (Variables|/Script/Engine.SceneComponent|GetRelativeLocation (Variables|Default|GetBox))) (Variables|Default|GetDestinationYValue))
      (Transformation|AddRelativeLocation (Variables|Default|GetBox) (Math|Vector|MakeVector 0.0 (Variables|Default|GetSpeed) 0.0) false false)
      (else
        (Variables|Default|SetOpening false)))
    (elif (Variables|Default|GetClosing)
      (if (>= (.y (Variables|/Script/Engine.SceneComponent|GetRelativeLocation (Variables|Default|GetBox))) (Variables|Default|GetFromLocationY))
        (Transformation|AddRelativeLocation (Variables|Default|GetBox) (Math|Vector|MakeVector 0.0 (* (Variables|Default|GetSpeed) -1.0) 0.0) false false)
        (else
          (Variables|Default|SetClosing false))))))

(event EventBeginPlay
  (Variables|Default|SetFromLocationY (.y (Variables|/Script/Engine.SceneComponent|GetRelativeLocation (Variables|Default|GetBox)))))

(fn ConstructionScript)