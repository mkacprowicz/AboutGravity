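; BP_GravLight is an indicator light Blueprint that shows red, yellow, white or black on its static mesh.
; It starts black on BeginPlay, and a separate event for each color swaps the material in slot 0.
; It holds no decision logic of its own, and nothing in its graph calls the color events.
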(event Custom|LightBlack
  (Rendering|Material|SetMaterial (Variables|Default|GetStaticMesh) 0 "/Game/StarterContent/Materials/M_Light_Black.M_Light_Black"))

(event Custom|LightRed
  (Rendering|Material|SetMaterial (Variables|Default|GetStaticMesh) 0 "/Game/StarterContent/Materials/M_Light_Red.M_Light_Red"))

(event Custom|LightYellow
  (Rendering|Material|SetMaterial (Variables|Default|GetStaticMesh) 0 "/Game/StarterContent/Materials/M_Light_Yellow.M_Light_Yellow"))

(event Custom|LightWhite
  (Rendering|Material|SetMaterial (Variables|Default|GetStaticMesh) 0 "/Game/StarterContent/Materials/M_Light_White.M_Light_White"))

(event EventBeginPlay
  (Rendering|Material|SetMaterial (Variables|Default|GetStaticMesh) 0 "/Game/StarterContent/Materials/M_Light_Black.M_Light_Black"))

(fn ConstructionScript)