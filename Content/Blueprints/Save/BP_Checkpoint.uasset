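; Checkpoint actor that saves player progress to the "check" slot when its Trigger is overlapped.
; With its Load flag on, it copies the player's location, health, ammo and gravity state into a loaded or newly created SaveAG via DataToSave, then destroys itself.
; With the flag off, it instead clears the existing save's Load flag, marking the checkpoint as cleared.
; Only the stat capture depends on the player cast; saving and clearing run for any overlapping actor.
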(event OnComponentBeginOverlap(Trigger)
  (params (OverlappedComponent :type Primitive%20Component%20Object%20Reference) (OtherActor :type Actor%20Object%20Reference) (OtherComp :type Primitive%20Component%20Object%20Reference) (OtherBodyIndex :type Integer) (bFromSweep :type Boolean) (SweepResult :type Hit%20Result%20Structure%20%28by%20ref%29))
  (if (Variables|Default|GetLoad)
    (Utilities|FlowControl|Sequence
      (:then_0
        (bind _asbp_player_character (Utilities|Casting|CastToBP_PlayerCharacter OtherActor))
        (Variables|Default|SetPlayerLocation (Transformation|GetActorLocation _asbp_player_character))
        (Variables|Default|SetPlayerHP (Variables|/Game/Blueprints/BP_PlayerCharacter.BP_PlayerCharacter_C|GetcurrPlayerHealth _asbp_player_character))
        (Variables|Default|SetPlayerAmmo (Variables|/Game/Blueprints/BP_PlayerCharacter.BP_PlayerCharacter_C|GetAmmo _asbp_player_character))
        (Variables|Default|SetPlayerGravState (Variables|/Game/Blueprints/BP_PlayerCharacter.BP_PlayerCharacter_C|GetGravityCharacterState _asbp_player_character)))
      (:then_1
        (bind _returnvalue (SaveGame|DoesSaveGameExist "check"))
        (if _returnvalue
          (bind _returnvalue_2 (SaveGame|LoadGamefromSlot "check"))
          (bind _assave_ag (Utilities|Casting|CastToSaveAG _returnvalue_2))
          (CallFunction|DatatoSave _assave_ag)
          (else
            (bind _returnvalue_3 (SaveGame|CreateSaveGameObject "/Game/Blueprints/Save/SaveAG.SaveAG_C"))
            (CallFunction|DatatoSave _returnvalue_3)))
        (Development|PrintString "Checkpoint" true true "(R=1.000000,G=1.000000,B=1.000000,A=1.000000)")
        (Utilities|FlowControl|Delay 0.2)
        (Actor|DestroyActor)))
    (else
      (bind _returnvalue_4 (SaveGame|LoadGamefromSlot "check"))
      (bind _assave_ag_2 (Utilities|Casting|CastToSaveAG _returnvalue_4))
      (Variables|/Game/Blueprints/Save/SaveAG.SaveAG_C|SetLoad _assave_ag_2 false)
      (SaveGame|SaveGametoSlot _assave_ag_2 "check")
      (Development|PrintString "CheckpointCleared"))))

(event EventBeginPlay)

(event Collision|EventActorBeginOverlap
  (params (OtherActor :type Actor%20Object%20Reference)))

(event EventTick
  (params (DeltaSeconds :type Float%20%28single-precision%29)))

(fn ConstructionScript)

(fn DatatoSave
  (params (SaveObj :type Save%20AG%20Object%20Reference))
  (LocalVariables|SetSaveObject SaveObj)
  (Variables|/Game/Blueprints/Save/SaveAG.SaveAG_C|SetPlayerLocation (LocalVariables|GetSaveObject) (Variables|Default|GetPlayerLocation))
  (Variables|/Game/Blueprints/Save/SaveAG.SaveAG_C|SetLoad (LocalVariables|GetSaveObject) true)
  (Variables|/Game/Blueprints/Save/SaveAG.SaveAG_C|SetPlayerHealth (LocalVariables|GetSaveObject) (Variables|Default|GetPlayerHP))
  (Variables|/Game/Blueprints/Save/SaveAG.SaveAG_C|SetPlayerAmmo (LocalVariables|GetSaveObject) (Variables|Default|GetPlayerAmmo))
  (Variables|/Game/Blueprints/Save/SaveAG.SaveAG_C|SetGravState (LocalVariables|GetSaveObject) (Variables|Default|GetPlayerGravState))
  (SaveGame|SaveGametoSlot (LocalVariables|GetSaveObject) "check")
  (return))