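; Death trigger actor that returns the player to their last saved checkpoint on contact.
; When BP_PlayerCharacter overlaps the Trigger, it disables input and waits two seconds.
; If the "check" save slot exists, it moves the player to the SaveAG's stored PlayerLocation and re-enables input.
; Otherwise, it opens the level named by its Level variable.
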(event OnComponentBeginOverlap(Trigger)
  (params (OverlappedComponent :type Primitive%20Component%20Object%20Reference) (OtherActor :type Actor%20Object%20Reference) (OtherComp :type Primitive%20Component%20Object%20Reference) (OtherBodyIndex :type Integer) (bFromSweep :type Boolean) (SweepResult :type Hit%20Result%20Structure%20%28by%20ref%29))
  (bind _asbp_player_character (Utilities|Casting|CastToBP_PlayerCharacter OtherActor))
  (Input|DisableInput _asbp_player_character (Game|GetPlayerController 0))
  (Utilities|FlowControl|Delay 2.0)
  (bind _returnvalue (SaveGame|DoesSaveGameExist "check"))
  (if _returnvalue
    (bind _returnvalue_2 (SaveGame|LoadGamefromSlot "check"))
    (bind _assave_ag (Utilities|Casting|CastToSaveAG _returnvalue_2))
    (bind _asbp_player_character_2 (Utilities|Casting|CastToBP_PlayerCharacter (Game|Player|GetPlayerPawn 0)))
    (Transformation|SetActorLocation _asbp_player_character_2 (Variables|/Game/Blueprints/Save/SaveAG.SaveAG_C|GetPlayerLocation _assave_ag) false false)
    (Input|EnableInput _asbp_player_character_2 (Game|GetPlayerController 0))
    (else
      (Game|OpenLevel(byName) (Variables|Default|GetLevel)))))

(event EventBeginPlay)

(event Collision|EventActorBeginOverlap
  (params (OtherActor :type Actor%20Object%20Reference)))

(event EventTick
  (params (DeltaSeconds :type Float%20%28single-precision%29)))

(fn ConstructionScript)