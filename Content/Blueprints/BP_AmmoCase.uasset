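; BP_AmmoCase is an ammo pickup that resupplies the player character when walked over.
; A box overlap casts to BP_PlayerCharacter, passes AmmoNum to ResupplyAmmo, then fires UsedEvent.
; UsedEvent flags the case as used, hides it, disables its collision and plays a pickup sound.
; Rather than being destroyed, the case can be restored by Renew, which clears the flag and re-enables visibility and collision.
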(event OnComponentBeginOverlap(Box)
  (params (OverlappedComponent :type Primitive%20Component%20Object%20Reference) (OtherActor :type Actor%20Object%20Reference) (OtherComp :type Primitive%20Component%20Object%20Reference) (OtherBodyIndex :type Integer) (bFromSweep :type Boolean) (SweepResult :type Hit%20Result%20Structure%20%28by%20ref%29))
  (bind _asbp_player_character (Utilities|Casting|CastToBP_PlayerCharacter OtherActor))
  (Default|ResupplyAmmo _asbp_player_character (Variables|Default|GetAmmoNum))
  (CallFunction|UsedEvent))

(event Custom|UsedEvent
  (Variables|Default|SetWasUsed true)
  (Rendering|SetActorHiddenInGame true)
  (Collision|SetActorEnableCollision false)
  (Audio|PlaySoundatLocation "/Game/AssetsPacks/SciFiWeapLight/Sound/Pistol/Wavs/Pistol_AmmoPickup02.Pistol_AmmoPickup02" (Transformation|GetActorLocation) "0, 0, 0" 1.0 1.0 0.0 0 0 0))

(event Custom|Renew
  (Variables|Default|SetWasUsed false)
  (Rendering|SetActorHiddenInGame false)
  (Collision|SetActorEnableCollision true))

(fn ConstructionScript)